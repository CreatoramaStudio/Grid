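; BP_SquareGridOutlinePainter is a grid painter Blueprint, named for outlining square grids.
; It adds no logic of its own: BeginPlay, UpdateGridState and TickImpl only forward to the parent class.
; GetColorPriority and GetColors likewise return the parent's results unchanged, so any painting behavior shown here is inherited.
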(event EventTickImpl
  (params (DeltaTime :type Float%20%28single-precision%29))
  (|CallParentFunction DeltaTime))

(event EventUpdateGridState
  (params (Grid :type Grid%20Object%20Reference))
  (|CallParentFunction Grid))

(event EventBeginPlay
  (|CallParentFunction))

(fn GetColorPriority
  (bind _colors (|CallParentFunction))
  (return _colors))

(fn GetColors
  (params (Grid :type Grid%20Object%20Reference))
  (bind _colors (|CallParentFunction Grid))
  (return _colors))